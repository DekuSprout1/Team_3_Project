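; Moving scaffolding-board platform that starts shuttling between its initial position and an EndPoint once a BP_PlayerCharacter carrying "Key" overlaps its Box.
; BeginPlay caches the start point and travel direction; Tick moves the boards at Speed without sweep while IsMoving is set.
; Direction flips whenever distance from the departure end exceeds the path length.
; GoingForward reads inverted: true drives movement back toward the start.
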(event OnComponentBeginOverlap(Box)
  (params (OverlappedComponent :type Primitive%20Component%20Object%20Reference) (OtherActor :type Actor%20Object%20Reference) (OtherComp :type Primitive%20Component%20Object%20Reference) (OtherBodyIndex :type Integer) (bFromSweep :type Boolean) (SweepResult :type Hit%20Result%20Structure%20%28by%20ref%29))
  (bind _asbp_player_character (Utilities|Casting|CastToBP_PlayerCharacter OtherActor))
  (if (Utilities|Array|ContainsItem (Variables|/Game/Blueprints/BP_PlayerCharacter.BP_PlayerCharacter_C|GetInventory%20 _asbp_player_character) "Key")
    (Variables|Default|SetIs%20Moving true)))

(event EventBeginPlay
  (Variables|Default|SetStart%20Point (Transformation|GetWorldLocation (Variables|Default|GetScaffoldingBridge_001_Boards)))
  (Variables|Default|SetMoveDirection (Math|Vector|GetUnitDirection(Vector) (Variables|Default|GetStart%20Point) (Transformation|GetWorldLocation (Variables|Default|GetEnd%20Point)))))

(event EventTick
  (params (DeltaSeconds :type Float%20%28single-precision%29))
  (if (Variables|Default|GetIs%20Moving)
    (Transformation|AddRelativeLocation (Variables|Default|GetScaffoldingBridge_001_Boards) (* (Variables|Default|GetMoveDirection) (* (Variables|Default|GetSpeed) (Math|Float|SelectFloat -1.0 1.0 (Variables|Default|GetGoing%20Forward)) DeltaSeconds)) false false)
    (if (> (Math|Vector|Distance(Vector) (Transformation|GetWorldLocation (Variables|Default|GetScaffoldingBridge_001_Boards)) (Math|Vector|SelectVector (Transformation|GetWorldLocation (Variables|Default|GetEnd%20Point)) (Variables|Default|GetStart%20Point) (Variables|Default|GetGoing%20Forward))) (Math|Vector|Distance(Vector) (Transformation|GetWorldLocation (Variables|Default|GetEnd%20Point)) (Variables|Default|GetStart%20Point)))
      (Variables|Default|SetGoing%20Forward (not (Variables|Default|GetGoing%20Forward))))))

(fn ConstructionScript)