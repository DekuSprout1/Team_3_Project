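; A collectable actor that the player picks up by walking into it.
; An overlap on its Box component by a BP_PlayerCharacter calls the Pickup event.
; Pickup decrements CollectablesLeft on BP_Gamemode, adds a newly created BP_Collectables widget to the viewport, then destroys the actor.
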(event OnComponentBeginOverlap(Box)
  (params (OverlappedComponent :type Primitive%20Component%20Object%20Reference) (OtherActor :type Actor%20Object%20Reference) (OtherComp :type Primitive%20Component%20Object%20Reference) (OtherBodyIndex :type Integer) (bFromSweep :type Boolean) (SweepResult :type Hit%20Result%20Structure%20%28by%20ref%29))
  (Utilities|Casting|CastToBP_PlayerCharacter OtherActor)
  (CallFunction|Pickup))

(event Custom|Pickup
  (bind _asbp_gamemode (Utilities|Casting|CastToBP_Gamemode (Game|GetGameMode)))
  (bind _result (Math|Integer|DecrementInt (Variables|/Game/Blueprints/BP_Gamemode.BP_Gamemode_C|GetCollectables%20Left _asbp_gamemode))
    (:%20%20
      (Variables|/Game/Blueprints/BP_Gamemode.BP_Gamemode_C|SetCollectables%20Left _asbp_gamemode _result)
      (bind _returnvalue (UserInterface|CreateWidget "/Game/UI/BP_Collectables.BP_Collectables_C"))
      (UserInterface|Viewport|AddtoViewport _returnvalue 0)
      (Actor|DestroyActor))))

(fn ConstructionScript)