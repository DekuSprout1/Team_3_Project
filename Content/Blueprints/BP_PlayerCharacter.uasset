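; BP_PlayerCharacter is the player character, handling side-to-side movement, jumping and opening the pause menu.
; Move_Left and Move_Right axes both add movement along the actor's right vector, scaled by the axis value, while the Jump action calls Jump.
; The Pause action creates a BP_JL_PauseMenu widget, adds it to the viewport, shows the mouse cursor and pauses the game.
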(event EventBeginPlay)

(event Collision|EventActorBeginOverlap
  (params (OtherActor :type Actor%20Object%20Reference)))

(event EventTick
  (params (DeltaSeconds :type Float%20%28single-precision%29)))

(event Input|ActionEvents|InputActionJump
  (params (Key :type Key%20Structure :default "None"))
  ;[1 1 1] Movment
  (:Pressed
    (Character|Jump)))

(event Input|ActionEvents|InputActionPause
  (params (Key :type Key%20Structure :default "None"))
  ;[1 1 1] Pause Menu
  (:Pressed
    (bind _returnvalue (UserInterface|CreateWidget "/Game/UI/BP_JL_PauseMenu.BP_JL_PauseMenu_C"))
    (UserInterface|Viewport|AddtoViewport _returnvalue 0)
    (Variables|/Script/Engine.PlayerController|SetbShowMouseCursor (Game|GetPlayerController 0) true)
    (Game|SetGamePaused true)))

(event Input|AxisEvents|InputAxisMove_Left
  (params (AxisValue :type Float%20%28single-precision%29))
  ;[1 1 1] Movment
  (Pawn|Input|AddMovementInput (Transformation|GetActorRightVector) AxisValue false))

(event Input|AxisEvents|InputAxisMove_Right
  (params (AxisValue :type Float%20%28single-precision%29))
  ;[1 1 1] Movment
  (Pawn|Input|AddMovementInput (Transformation|GetActorRightVector) AxisValue false))

(fn ConstructionScript)