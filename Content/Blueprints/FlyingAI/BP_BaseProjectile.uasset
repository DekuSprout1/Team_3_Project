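; Base projectile actor in the FlyingAI folder that moves via ProjectileMovement and damages the player.
; Construction applies configurable speed, gravity, lifespan and bullet material.
; A looping timer sphere-traces from the previous location to slightly ahead, scaled by velocity, instead of using collision events.
; Any hit subtracts fixed health from player 0, regardless of what was struck, destroys the projectile and calls the controller's OnDeath at zero health.
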(event Custom|Tick
  (bind _returnvalue (Collision|SphereTraceForObjects (Variables|Default|GetPreviousLocation) (+ (Transformation|GetActorLocation) (* (Transformation|GetActorForwardVector) (* (Math|Vector|VectorLength (Variables|/Script/Engine.MovementComponent|GetVelocity (Variables|Default|GetProjectileMovement))) (Variables|Default|GetTraceTickerate) 0.5))) (Variables|Default|GetRadius) (Utilities|Array|MakeArray "ObjectTypeQuery1" "ObjectTypeQuery2" "ObjectTypeQuery3") false (Variables|Default|GetIgnoredActors) "None"))
  (if _returnvalue
    (bind _asbp_player_character (Utilities|Casting|CastToBP_PlayerCharacter (Game|GetPlayerCharacter 0)))
    (bind _output_get (Variables|/Game/Blueprints/BP_PlayerCharacter.BP_PlayerCharacter_C|SetCurrentHealth _asbp_player_character (- (Variables|/Game/Blueprints/BP_PlayerCharacter.BP_PlayerCharacter_C|GetCurrentHealth _asbp_player_character) 2.0)))
    (Actor|DestroyActor)
    (if (<= _output_get 0.0)
      (bind _asbp_player_controller (Utilities|Casting|CastToBP_PlayerController (Pawn|GetController _asbp_player_character)))
      (Default|OnDeath _asbp_player_controller))
    (else
      (Variables|Default|SetPreviousLocation (Transformation|GetActorLocation)))))

(event EventBeginPlay
  (bind _returnvalue (Utilities|Time|SetTimerbyEvent (delegate Custom|Tick) (Variables|Default|GetTraceTickerate) true))
  (Variables|Default|SetTraceTimer _returnvalue))

(fn ConstructionScript
  (bind _projectilemovement (Variables|Default|GetProjectileMovement))
  (bind _speed (Variables|Default|GetSpeed))
  (Variables|Default|SetPreviousLocation (Transformation|GetActorLocation))
  (Actor|SetLifeSpan (Variables|Default|GetLifespan))
  (Variables|/Script/Engine.ProjectileMovementComponent|SetInitialSpeed _projectilemovement _speed)
  (Variables|/Script/Engine.ProjectileMovementComponent|SetMaxSpeed _projectilemovement _speed)
  (Variables|/Script/Engine.ProjectileMovementComponent|SetProjectileGravityScale _projectilemovement (Variables|Default|GetGravity))
  (Rendering|Material|SetMaterial (Variables|Default|Getbullet) 0 (Variables|Default|GetMaterial)))