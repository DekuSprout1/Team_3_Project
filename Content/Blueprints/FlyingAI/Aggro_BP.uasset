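; Flying AI pawn that patrols placed points, chases the player on sight and searches when sight is lost.
; Two looping timers replace Tick: one detects the player by dot-product view cone and line trace, the other runs movement for the current FlyingMode.
; FloatingPawnMovement drives it forward while interpolated rotation steers toward the patrol point or last seen location.
; Searching spins it one full turn at that location before resuming patrol.
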(event Custom|MovementTick
  ;[1 1 1] Movement tick
  (switch Utilities|FlowControl|Switch|SwitchonE_AggroFlyingMode (Variables|Movement|GetFlyingMode)
    (:NewEnumerator0
      (CallFunction|PatrolMovement))
    (:NewEnumerator1
      (CallFunction|AggroMovement))
    (:NewEnumerator2
      (CallFunction|LFPMovement))))

(event Custom|CheckForPlayer
  ;[1 1 1] Find and line trace player
  ;;[1 1 1] Movement tick
  (bind (_location _foundplayer_) (CallFunction|TraceforPlayer))
  (if _foundplayer_
    (Variables|Aggro|SetLastSawPlayerLocation _location)
    (Variables|Movement|SetFlyingMode "NewEnumerator1")
    (else
      (switch Utilities|FlowControl|Switch|SwitchonE_AggroFlyingMode (Variables|Movement|GetFlyingMode)
        (:NewEnumerator1
          (Variables|Movement|SetFlyingMode "NewEnumerator2")
          (Variables|Default|SetLookingForPlayerCounter 0))))))

(event Custom|PatrolMovement
  (bind _patrol_points (Variables|Patrol|GetPatrol%20Points))
  (bind _patrolindex (Variables|Patrol|GetPatrolIndex))
  (bind _output (Utilities|Array|Get(acopy) _patrol_points _patrolindex))
  ;[1 1 1] Patrol
  (if (Variables|Patrol|GetCan%20Patrol)
    (if (< (Transformation|GetDistanceTo self _output) (Variables|Patrol|GetPatrolAcceptanceRadius))
      (CallFunction|GetNextPatrolLocation)
      (else
        (CallFunction|DoMovementTick true true (Transformation|GetActorLocation _output))))))

(event Custom|LFPMovement
  ;[1 1 1] Looking for player movement
  (if (> (Math|Vector|VectorLength (- (Transformation|GetActorLocation) (Variables|Aggro|GetLastSawPlayerLocation))) (Variables|Default|GetAggroAcceptanceRadius))
    (CallFunction|DoMovementTick true true (Variables|Aggro|GetLastSawPlayerLocation))
    (else
      (Variables|/Script/Engine.MovementComponent|SetVelocity (Variables|Default|GetFloatingPawnMovement) "0, 0, 0")
      (bind _result (Math|Integer|IncrementInt (Variables|Default|GetLookingForPlayerCounter))
        (:%20%20
          (if (> _result (Variables|Default|GetMaxLFP))
            (Variables|Movement|SetFlyingMode "NewEnumerator0")
            (else
              (Class|Actor|AddActorWorldRotation (Math|Rotator|MakeRotator 0.0 0.0 (/ 3.6e+02 (Math|Conversions|ToFloat(Integer) (Variables|Default|GetMaxLFP))))))))))))

(event Custom|DoMovementTick
  (params (DoForwardMovement :type Boolean) (DoRotation :type Boolean) (location :type Vector))
  (bind _aggrorinterpspeed (Variables|Aggro|GetAggroRinterpSpeed))
  (bind _aggromovespeed (Variables|Aggro|GetAggroMoveSpeed))
  (Utilities|FlowControl|Sequence
    (:then_0
      ;[1 1 1] Movement speed
      (if DoForwardMovement
        (Class|PawnMovementComponent|AddInputVector (Variables|Default|GetFloatingPawnMovement) (* (Transformation|GetActorForwardVector) (Utilities|Select :Index (Variables|Movement|GetFlyingMode) :NewEnumerator0 (Variables|Patrol|GetPatrolMoveSpeed) :NewEnumerator1 _aggromovespeed :NewEnumerator2 _aggromovespeed)) false)))
    (:then_1
      ;[1 1 1] Rotation
      (if DoRotation
        (Transformation|SetActorRotation (Math|Interpolation|RInterpTo (Transformation|GetActorRotation) (Math|Conversions|RotationFromXVector (Math|Vector|Normalize (- location (Transformation|GetActorLocation)))) (Variables|Movement|GetMovementTickRate) (Utilities|Select :Index (Variables|Movement|GetFlyingMode) :NewEnumerator0 (Variables|Patrol|GetPatrolRinterpSpeed) :NewEnumerator1 _aggrorinterpspeed :NewEnumerator2 _aggrorinterpspeed)))))))

(event Custom|AggroMovement
  ;[1 1 1] Aggro movement
  (if (> (Math|Vector|VectorLength (- (Transformation|GetActorLocation) (Variables|Aggro|GetLastSawPlayerLocation))) (Variables|Default|GetAggroAcceptanceRadius))
    (CallFunction|DoMovementTick true true (Variables|Aggro|GetLastSawPlayerLocation))
    (else
      (CallFunction|DoMovementTick false true (Variables|Aggro|GetLastSawPlayerLocation))
      (Variables|/Script/Engine.MovementComponent|SetVelocity (Variables|Default|GetFloatingPawnMovement) "0, 0, 0"))))

(event EventBeginPlay
  ;[1 1 1] Movement tick
  (CallFunction|CheckCanPatrol)
  (bind _returnvalue (Utilities|Time|SetTimerbyEvent (delegate Custom|MovementTick) (Variables|Movement|GetMovementTickRate) true))
  (Variables|Movement|SetMovementTimer _returnvalue)
  (bind _returnvalue_2 (Utilities|Time|SetTimerbyEvent (delegate Custom|CheckForPlayer) (Variables|CheckForPlayer|GetCheckForPlayerTick) true))
  (Variables|CheckForPlayer|SetCheckForPlayerTimer _returnvalue_2))

(fn ConstructionScript)

(fn CheckCanPatrol
  ;[1 1 1] If length of patrol points is greater than 0 then true
  (if (> (Utilities|Array|Length (Variables|Patrol|GetPatrol%20Points)) 0)
    ;[1 1 1] Loops throw patrol points array to see if they are valid and wether can petrol or not
    (for _array_element (Variables|Patrol|GetPatrol%20Points)
      (Utilities|IsValid _array_element
        (:Is%20Not%20Valid
          (Math|Integer|IncrementInt (LocalVariables|GetInvalidIndexes)))))
    (Variables|Patrol|SetCan%20Patrol (not (== (LocalVariables|GetInvalidIndexes) (Utilities|Array|Length (Variables|Patrol|GetPatrol%20Points)))))
    (else
      (Variables|Patrol|SetCan%20Patrol false))))

(fn GetNextPatrolLocation
  (bind _output_get (Variables|Patrol|SetPatrolIndex (Math|Integer|SelectInt 0 (+ (Variables|Patrol|GetPatrolIndex) 1) (== (+ (Variables|Patrol|GetPatrolIndex) 1) (Utilities|Array|Length (Variables|Patrol|GetPatrol%20Points)))) :!label _label))
  (Utilities|IsValid (Utilities|Array|Get(acopy) (Variables|Patrol|GetPatrol%20Points) _output_get)
    (:Is%20Not%20Valid
      (goto _label))))

(fn TraceforPlayer
  (bind _returnvalue (Game|GetPlayerCharacter 0))
  (bind _returnvalue_2 (Transformation|GetActorLocation))
  (bind _arrow (Variables|Default|GetArrow))
  (bind _returnvalue_3 (Transformation|GetActorLocation _returnvalue))
  (bind _returnvalue_4 (Transformation|GetWorldLocation _arrow))
  (bind _returnvalue_5 (- _returnvalue_3 _returnvalue_2))
  (bind _returnvalue_6 (Math|Vector|Normalize _returnvalue_5))
  (if (> (Math|Vector|DotProduct (Math|Vector|GetForwardVector (Variables|Default|GetArrow)) _returnvalue_6) (Variables|CheckforPlayer|GetFindPlayerDot))
    (bind (_outhit _returnvalue_7) (Collision|LineTraceForObjects _returnvalue_4 (+ _returnvalue_4 (* _returnvalue_6 (Variables|CheckforPlayer|GetPlayerTraceDistance))) (Utilities|Array|MakeArray "ObjectTypeQuery1" "ObjectTypeQuery2" "ObjectTypeQuery3" "ObjectTypeQuery4" "ObjectTypeQuery6") false 0 (select (Variables|Aggro|GetTraceDebug) "ForDuration" "None")))
    (if _returnvalue_7
      (return (.ImpactPoint (Collision|BreakHitResult _outhit)) (== (.HitActor (Collision|BreakHitResult _outhit)) (Game|GetPlayerCharacter 0)))
      (else
        (return "0, 0, 0" false)))
    (else
      (return "0, 0, 0" false))))